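; Zombie actor that seeks out targets and responds to player-issued move and flee commands, moving via AIMoveTo.
; TargetCancelled picks the highest-value tagged actor by BP_Component_Target, skipping the last one reached, and notifies that component, or wanders randomly when none qualifies.
; Short-range and flee events act only within ShortRangeDistance, then search again; flee picks a random point around the flee location.
; Long-range orders move near a BP_BrainZombieTarget and trigger IsBeingEaten.
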(event `self.ReceiveBeginPlay`
  (bind _output_get (set `self.Target` self))
  (set `self.PastTarget` _output_get)
  (`self.TargetCancelled`))

(event `self.ReceiveTick`
  (params (DeltaSeconds :type "Float (single-precision)")))

(event `SetNewTarget`
  (params (NewTarget :type "Actor Object Reference")))

(event `RegisterShortRange`
  (params (Location :type "Transform Structure"))
  (bind _returnvalue (`KismetMathLibrary.TransformLocation` Location))
  ; Short Range Player Direction - Zombie checks if within range, then moves to location
  (`KismetSystemLibrary.PrintString` "short range called")
  (if (<= (`KismetMathLibrary.Vector_Distance` _returnvalue (`KismetMathLibrary.TransformLocation` (`self.GetTransform` self))) (`self.ShortRangeDistance`))
    (`|AIMoveTo` self _returnvalue null
      (:`then`
        (`KismetSystemLibrary.PrintString` "short range move"))
      (:`OnSuccess`
        (`self.TargetCancelled` :!label _label))
      (:`OnFail`
        (goto _label)))))

(event `RegisterLongRange`
  (params (Location :type "Transform Structure") (Target :type "Actor Object Reference"))
  ; Long Range Player Directioin - Zombie moves to location, starts "eating" target
  (`KismetSystemLibrary.PrintString` "long range called")
  (`|AIMoveTo` self (`NavigationSystemV1.K2_GetRandomReachablePointInRadius` (`self.K2_GetActorLocation` Target) 200.0 null null) null 200.0
    (:`then`
      (`KismetSystemLibrary.PrintString` "long range move"))
    (:`OnSuccess`
      (bind _asbp_brain_zombie_target (cast `/Game/BP_BrainZombieTarget` Target))
      (`/Game/BP_BrainZombieTarget.IsBeingEaten` _asbp_brain_zombie_target))
    (:`OnFail`
      (`KismetSystemLibrary.PrintString` "long range failed"))))

(event `TargetCancelled`
  (bind _target (`self.Target`))
  (bind _target_2 (`self.Target`))
  (bind _returnvalue (`self.GetComponentByClass` _target_2 "/Game/BP_Component_Target.BP_Component_Target_C"))
  (bind _returnvalue_2 (`self.GetComponentByClass` (`self.Target`) "/Game/BP_Component_Target.BP_Component_Target_C"))
  (bind _returnvalue_3 (`ActorComponent.GetOwner` (`Actor.RootComponent` _target)))
  (bind _value (`/Game/BP_Component_Target.Value` _returnvalue_2))
  ; Target has been deleted - idle(?) and search for new target
  (`KismetSystemLibrary.PrintString` "search called")
  (bind _outactors (`GameplayStatics.GetAllActorsWithTag` "\"Target\""))
  (if (== (`KismetArrayLibrary.Array_Length` _outactors) 0)
    (`KismetSystemLibrary.PrintString` "zombie target" :!label _label_2)
    (`|AIMoveTo` self (`NavigationSystemV1.K2_GetRandomReachablePointInRadius` (`self.K2_GetActorLocation` self) 600.0 null null) null
      (:`OnSuccess`
        _)
      (:`OnFail`
        _))
    (`self.TargetCancelled`)
    (else
      (`KismetArrayLibrary.Array_RemoveItem` _outactors (`self.Target`))
      (set `self.Target` self)
      (`KismetSystemLibrary.PrintString` (`KismetStringLibrary.Conv_IntToString` (`KismetArrayLibrary.Array_Length` _outactors)))
      (for (_array_element _array_index) _outactors
        (`KismetSystemLibrary.PrintString` (`KismetStringLibrary.Conv_IntToString` _array_index))
        (if (!= (`self.PastTarget`) _array_element)
          (bind _returnvalue_4 (`self.GetComponentByClass` _array_element "/Game/BP_Component_Target.BP_Component_Target_C"))
          (bind _value_2 (`/Game/BP_Component_Target.Value` _returnvalue_4))
          (if (> _value_2 _value)
            (bind _output_get (set `self.Target` _array_element))
            (`KismetSystemLibrary.PrintString` (`KismetSystemLibrary.GetDisplayName` _output_get))
            (`KismetSystemLibrary.PrintString` "target set as ^")
            (else
              (`KismetSystemLibrary.PrintString` "not added, val:")
              (`KismetSystemLibrary.PrintString` (`KismetStringLibrary.Concat_StrStr` (`KismetSystemLibrary.GetDisplayName` _returnvalue_4) (`KismetStringLibrary.Conv_DoubleToString` _value_2) "<" (`KismetSystemLibrary.GetDisplayName` _returnvalue_2) (`KismetStringLibrary.Conv_DoubleToString` _value)))))
          (else
            (`KismetSystemLibrary.PrintString` "unv target"))))
      (if (!= self _target)
        (`KismetSystemLibrary.PrintString` (`KismetStringLibrary.Concat_StrStr` "moving towards: " (`KismetSystemLibrary.GetDisplayName` _target)))
        (cast `/Game/BP_Zombie2` (`self.Target`)
          (:`then`
            (goto _label_2))
          (:`CastFailed`
            (`|AIMoveTo` self (`NavigationSystemV1.K2_GetRandomReachablePointInRadius` (`self.K2_GetActorLocation` _returnvalue_3) 200.0 null null) _returnvalue_3 50.0
              (:`then`
                (`/Game/BP_Component_Target.SetTargetOf` _returnvalue self))
              (:`OnSuccess`
                (`KismetSystemLibrary.PrintString` (`KismetStringLibrary.Concat_StrStr` "\"reached target: \"" (`KismetSystemLibrary.GetDisplayName` _target_2)))
                (`/Engine/EditorBlueprintResources/StandardMacros.IsValid` _target_2
                  (:`Is Valid`
                    (`/Game/BP_Component_Target.TargetReached` _returnvalue)
                    (set `self.PastTarget` _target_2))))
              (:`OnFail`
                (`KismetSystemLibrary.PrintString` "failed to reach target")))))
        (else
          (`KismetSystemLibrary.PrintString` "no valid target")
          (goto _label_2))))))

(event `FleeFromPoint`
  (params (FleePoint :type "Transform Structure"))
  (bind _returnvalue (`KismetMathLibrary.TransformLocation` FleePoint))
  ; Flee from Point
  (`KismetSystemLibrary.PrintString` "short range called")
  (if (<= (`KismetMathLibrary.Vector_Distance` _returnvalue (`KismetMathLibrary.TransformLocation` (`self.GetTransform` self))) (`self.ShortRangeDistance`))
    (bind _randomlocation (`NavigationSystemV1.K2_GetRandomLocationInNavigableRadius` _returnvalue 1000.0 null null))
    (`|AIMoveTo` self _randomlocation null
      (:`OnSuccess`
        _)
      (:`OnFail`
        _))
    (`self.TargetCancelled`)))

(fn `UserConstructionScript`)