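; BP_Zombie is a player-directed zombie that walks to commanded locations or targets using AI MoveTo.
; Short-range orders apply only within ShortRangeDistance; long-range orders send it to a BP_BrainZombieTarget, calling IsBeingEaten on arrival, and both set UnderPlayerDirection.
; SetNewTarget follows a BP_Component_Target's owner, and TargetCancelled rescans "Target"-tagged actors, comparing component Value to retarget.
; BeginPlay and right-click trigger test moves, with debug prints throughout.
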(event `self.ReceiveBeginPlay`
  (bind _returnvalue (`GameplayStatics.GetActorOfClass` "/Game/TopDown/Blueprints/BP_TopDownCharacter.BP_TopDownCharacter_C"))
  (`KismetSystemLibrary.PrintString` (`KismetSystemLibrary.GetDisplayName` _returnvalue))
  (`|AIMoveTo` self (+ (`self.K2_GetActorLocation` self) (500.0 0.0 0.0)) null
    (:`then`
      (`KismetSystemLibrary.PrintString` "1move"))
    (:`OnFail`
      (`KismetSystemLibrary.PrintString` "1movefail"))))

(event `self.ReceiveTick`
  (params (DeltaSeconds :type "Float (single-precision)")))

(event `SetNewTarget`
  (params (NewTarget :type "Object Object Reference"))
  (bind _asbp_component_target (cast `/Game/Blueprints/BP_Component_Target` NewTarget))
  (bind _output_get (set `self.Target` _asbp_component_target))
  (`|AIMoveTo` self (0.0 0.0 0.0) (`ActorComponent.GetOwner` _output_get)))

(event `RegisterShortRange`
  (params (Location :type "Transform Structure"))
  (bind _returnvalue (`KismetMathLibrary.TransformLocation` Location))
  ; Short Range Player Direction - Zombie checks if within range, then moves to location
  (`KismetSystemLibrary.PrintString` "shor range called")
  (if (<= (`KismetMathLibrary.Vector_Distance` _returnvalue (`KismetMathLibrary.TransformLocation` (`self.GetTransform` self))) (`self.ShortRangeDistance`))
    (set `self.UnderPlayerDirection` true)
    (`|AIMoveTo` self _returnvalue null
      (:`then`
        (`KismetSystemLibrary.PrintString` "short range move"))
      (:`OnSuccess`
        (set `self.UnderPlayerDirection` false :!label _label))
      (:`OnFail`
        (goto _label)))))

(event `RegisterLongRange`
  (params (Location :type "Transform Structure") (Target :type "Object Object Reference"))
  ; Long Range Player Directioin - Zombie moves to location, starts "eating" target
  (`KismetSystemLibrary.PrintString` "long range called")
  (bind _asbp_brain_zombie_target (cast `/Game/Blueprints/BP_BrainZombieTarget` Target))
  (set `self.UnderPlayerDirection` true)
  (`|AIMoveTo` self (0.0 0.0 0.0) _asbp_brain_zombie_target
    (:`then`
      (`KismetSystemLibrary.PrintString` "long range move"))
    (:`OnSuccess`
      (`/Game/Blueprints/BP_BrainZombieTarget.IsBeingEaten` _asbp_brain_zombie_target)
      (set `self.UnderPlayerDirection` false :!label _label_2))
    (:`OnFail`
      (`KismetSystemLibrary.PrintString` "\"failed\"")
      (goto _label_2))))

(event `TargetCancelled`
  (bind _target (`self.Target`))
  (bind _target_2 (`self.Target`))
  ; Target has been deleted - idle(?) and search for new target
  (set `self.UnderPlayerDirection` false)
  (bind _outactors (`GameplayStatics.GetAllActorsWithTag` "\"Target\""))
  (`KismetSystemLibrary.PrintString` (`KismetStringLibrary.Conv_IntToString` (`KismetArrayLibrary.Array_Length` _outactors)))
  (for _array_element _outactors
    (bind _returnvalue (`self.GetComponentByClass` _array_element "/Game/Blueprints/BP_Component_Target.BP_Component_Target_C"))
    (`/Engine/EditorBlueprintResources/StandardMacros.IsValid` _returnvalue
      (:`Is Valid`
        (`KismetSystemLibrary.PrintString` (`KismetSystemLibrary.GetDisplayName` _target))
        (if (>= (`/Game/Blueprints/BP_Component_Target.Value` _returnvalue) (`/Game/Blueprints/BP_Component_Target.Value` _target))
          (set `self.Target` _returnvalue :!label _label_3)))
      (:`Is Not Valid`
        (goto _label_3))))
  (`/Engine/EditorBlueprintResources/StandardMacros.IsValid` _target_2
    (:`Is Valid`
      (`|AIMoveTo` self (0.0 0.0 0.0) (`ActorComponent.GetOwner` _target_2)))
    (:`Is Not Valid`
      (`KismetSystemLibrary.PrintString` "no valid target"))))

(event `Key|RightMouseButton`
  (params (Key :type "Key Structure"))
  (:`Pressed`
    (`KismetSystemLibrary.PrintString` "register click")
    (bind _returnvalue (`GameplayStatics.GetActorOfClass` "/Game/TopDown/Blueprints/BP_TopDownCharacter.BP_TopDownCharacter_C"))
    (`|AIMoveTo` self (0.0 0.0 0.0) _returnvalue
      (:`then`
        (`KismetSystemLibrary.PrintString` "\"trying\"")))))

(fn `UserConstructionScript`)