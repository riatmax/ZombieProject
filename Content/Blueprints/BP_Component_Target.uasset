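; BP_Component_Target is an actor component that marks its owner as something zombies can hunt.
; It tracks targeters in a Targeting array and, on NPC owners, updates pursuers and switches between Flee and Wander as they die.
; When reached, it blocks further targeting, cancels every pursuer's target, and destroys non-BP_Zombie2 owners.
; If flagged IsFinal, it resets the game through BP_FinalTarget as a win instead of destroying the owner.
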(event `self.ReceiveBeginPlay`
  (set `self.CanBeTargeted` true))

(event `SetTargetOf`
  (params (Targeter :type "/Game/TopDown/Blueprints/BP_Zombie2 Object Reference"))
  (bind _targeting (`self.Targeting`))
  ; Logs which zombies are in pursuit
  (if (`self.CanBeTargeted`)
    (`KismetArrayLibrary.Array_Add` _targeting Targeter)
    (bind _asbp_npc (cast `/Game/TopDown/Blueprints/BP_NPC` (`self.GetOwner`)))
    (`/Game/TopDown/Blueprints/BP_NPC.AddToPursuers` _asbp_npc _targeting)))

(event `TargetReached`
  ; When zombie reaches target, have pursuers retarget and self destruct
  (set `self.CanBeTargeted` false)
  (`KismetSystemLibrary.PrintText` "array length")
  (for _array_element (`self.Targeting`)
    (`/Game/TopDown/Blueprints/BP_Zombie2.TargetCancelled` _array_element))
  (cast `/Game/TopDown/Blueprints/BP_Zombie2` (`self.GetOwner`)
    (:`CastFailed`
      (`self.SelfDestruct`))))

(event `SelfDestruct`
  (bind _returnvalue (`self.GetOwner`))
  ; Destroys self after being eaten by zombie
  (`KismetSystemLibrary.PrintString` "\"Target Self Destruct!\"")
  (if (`self.IsFinal`)
    (`KismetSystemLibrary.PrintString` "Game Won!")
    (`/Game/BP_FinalTarget.ResetGame` (`Actor.GetComponentByClass` _returnvalue "/Game/BP_FinalTarget.BP_FinalTarget_C"))
    (else
      (`Actor.K2_DestroyActor` _returnvalue))))

(event `PursuerDied`
  (params (targeter :type "/Game/TopDown/Blueprints/BP_Zombie2 Object Reference"))
  ; Register that a pursuer has died
  (`KismetArrayLibrary.Array_RemoveItem` (`self.Targeting`) targeter)
  (bind _asbp_npc (cast `/Game/TopDown/Blueprints/BP_NPC` (`self.GetOwner`)))
  (`/Game/TopDown/Blueprints/BP_NPC.TargeterDied` _asbp_npc targeter)
  (if (== 0 (`KismetArrayLibrary.Array_Length` (`self.Targeting`)))
    (`/Game/TopDown/Blueprints/BP_NPC.Wander` _asbp_npc)
    (else
      (`/Game/TopDown/Blueprints/BP_NPC.Flee` _asbp_npc))))