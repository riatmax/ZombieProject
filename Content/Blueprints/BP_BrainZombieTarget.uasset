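; BP_BrainZombieTarget is a brain lure that draws zombies to itself and is eaten once they reach it.
; On BeginPlay it registers itself as a long-range target with every BP_Zombie2 in the level.
; IsBeingEaten, meant to be called when a zombie arrives, starts a Tick timer.
; When EatingLasts elapses, it destroys its target component, cancels the target on all zombies and destroys itself.
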(event `self.ReceiveBeginPlay`
  ; When spawned, call all zombies to location
  (bind _outactors (`GameplayStatics.GetAllActorsOfClass` "/Game/TopDown/Blueprints/BP_Zombie2.BP_Zombie2_C"))
  (for _array_element _outactors
    (`/Game/TopDown/Blueprints/BP_Zombie2.RegisterLongRange` :`self` _array_element :`Target` self)
    (set `self.BeingEaten` false))
  (`KismetSystemLibrary.PrintString` "\"logged\""))

(event `self.ReceiveTick`
  (params (DeltaSeconds :type "Float (single-precision)"))
  ; Counts down to destruction when first zombies have reached self
  (if (`self.BeingEaten`)
    (bind _output_get (set `self.SecondsEaten` (+ DeltaSeconds (`self.SecondsEaten`))))
    (if (>= _output_get (`self.EatingLasts`))
      (`ActorComponent.K2_DestroyComponent` (`self.BP_Component_Target`))
      (bind _outactors (`GameplayStatics.GetAllActorsOfClass` "/Game/TopDown/Blueprints/BP_Zombie2.BP_Zombie2_C"))
      (for _array_element _outactors
        (`/Game/TopDown/Blueprints/BP_Zombie2.TargetCancelled` _array_element))
      (`KismetSystemLibrary.PrintString` "\"eaten\"")
      (`self.K2_DestroyActor`))))

(event `IsBeingEaten`
  ; Called when zombie reaches self, starts destruction countdown
  (set `self.BeingEaten` true)
  (`KismetSystemLibrary.PrintString` "\"Eating!\""))

(fn `UserConstructionScript`)