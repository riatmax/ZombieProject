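; BP_FinalTarget keeps track of the living zombies and restarts the game once they are all dead.
; AddZombie and ZombieDied add and remove entries in the TheZombies array, printing a debug message each time.
; When a death leaves the array empty, ResetGame prints a message and opens the Landscape level by name.
; BeginPlay and Tick are unused.
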(event `ResetGame`
  (`KismetSystemLibrary.PrintString` "\"reset?\"")
  (`GameplayStatics.OpenLevel` "Landscape"))

(event `AddZombie`
  (params (Zombie :type "/Game/TopDown/Blueprints/BP_Zombie2 Object Reference"))
  (`KismetArrayLibrary.Array_Add` (`self.TheZombies`) Zombie)
  (`KismetSystemLibrary.PrintString` "zombie added"))

(event `ZombieDied`
  (params (Zombie :type "/Game/TopDown/Blueprints/BP_Zombie2 Object Reference"))
  (bind _thezombies (`self.TheZombies`))
  (`KismetArrayLibrary.Array_RemoveItem` _thezombies Zombie)
  (`KismetSystemLibrary.PrintString` "zombie died")
  (if (<= (`KismetArrayLibrary.Array_Length` _thezombies) 0)
    (`self.ResetGame`)))