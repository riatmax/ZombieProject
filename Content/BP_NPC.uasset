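; NPC Blueprint that wanders the navmesh until it has pursuers, then flees from them using AI MoveTo.
; Wander loops through random nearby points while the InPursuit array is empty.
; AddToPuruers replaces that array and calls Flee, which Tick and move completion also retrigger, targeting near the pursuers' negated, scaled average world position.
; FleeFromPoint moves to a random spot around a supplied point when within short range.
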(event `self.ReceiveBeginPlay`
  (`self.Wander`))

(event `self.ReceiveTick`
  (params (DeltaSeconds :type "Float (single-precision)"))
  (if (!= (`KismetArrayLibrary.Array_Length` (`self.InPursuit`)) 0)
    (`self.Flee`)))

(event `Wander`
  ; NPC wanders before being targeted
  (bind _randomlocation (`NavigationSystemV1.K2_GetRandomLocationInNavigableRadius` (`self.K2_GetActorLocation` self) 400.0 null null))
  (`|AIMoveTo` self _randomlocation null 10.0
    (:`OnSuccess`
      _)
    (:`OnFail`
      _))
  (if (== (`KismetArrayLibrary.Array_Length` (`self.InPursuit`)) 0)
    (`self.Wander`)))

(event `Flee`
  (bind _inpursuit (`self.InPursuit`))
  (`KismetSystemLibrary.PrintString` "FLEE")
  (set `self.FlightDirection` (0.0 0.0 0.0))
  (for _array_element _inpursuit
    (set `self.FlightDirection` (+ (`self.FlightDirection`) (`self.K2_GetActorLocation` _array_element))))
  (bind _output_get (set `self.FlightDirection` (* (`KismetMathLibrary.NegateVector` (/ (`self.FlightDirection`) (`KismetArrayLibrary.Array_Length` _inpursuit))) (1000.0 1000.0 1000.0))))
  (bind _randomlocation (`NavigationSystemV1.K2_GetRandomLocationInNavigableRadius` _output_get 200.0 null null))
  (`|AIMoveTo` self _randomlocation null
    (:`OnSuccess`
      _)
    (:`OnFail`
      _))
  (`self.Flee`))

(event `FleeFromPoint`
  (params (FleePoint :type "Transform Structure"))
  (bind _returnvalue (`KismetMathLibrary.TransformLocation` FleePoint))
  ; Flee from Point
  (`KismetSystemLibrary.PrintString` "short range called")
  (if (<= (`KismetMathLibrary.Vector_Distance` _returnvalue (`KismetMathLibrary.TransformLocation` (`self.GetTransform` self))) (`self.ShortRangeDistance`))
    (bind _randomlocation (`NavigationSystemV1.K2_GetRandomLocationInNavigableRadius` _returnvalue 1000.0 null null))
    (`|AIMoveTo` self _randomlocation null)))

(event `AddToPuruers`
  (params (NewTargeters :type "Array of /Game/BP_Zombie2 Object Reference"))
  (set `self.InPursuit` NewTargeters)
  (`self.Flee`))

(fn `UserConstructionScript`)