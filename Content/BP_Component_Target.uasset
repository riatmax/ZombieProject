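; BP_Component_Target is a component that marks its owning actor as a target and tracks who is targeting it.
; SetTargetOf adds each targeter to a Targeting array while the CanBeTargeted flag is set.
; TargetReached clears the flag, calls TargetCancelled on every stored targeter, then destroys the owning actor through SelfDestruct, with debug prints along the way.
; CheckTarget only branches on the flag and does nothing further.
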(event `self.ReceiveBeginPlay`
  (set `self.CanBeTargeted` true))

(event `SetTargetOf`
  (params (Targeter :type "/Game/TopDown/Blueprints/BP_Zombie2 Object Reference"))
  (if (`self.CanBeTargeted`)
    (`KismetArrayLibrary.Array_Add` (`self.Targeting`) Targeter)))

(event `TargetReached`
  (bind _targeting (`self.Targeting`))
  (set `self.CanBeTargeted` false)
  (`KismetSystemLibrary.PrintText` "array length")
  (`KismetSystemLibrary.PrintString` (`KismetStringLibrary.Conv_IntToString` (`KismetArrayLibrary.Array_Length` _targeting)))
  (for _array_element _targeting
    (`/Game/TopDown/Blueprints/BP_Zombie2.TargetCancelled` _array_element))
  (`self.SelfDestruct`))

(event `SelfDestruct`
  (`KismetSystemLibrary.PrintString` "\"Target Self Destruct!\"")
  (`Actor.K2_DestroyActor` (`self.GetOwner`)))

(event `CheckTarget`
  (if (`self.CanBeTargeted`)
    _))